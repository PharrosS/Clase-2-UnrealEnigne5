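; Teleporter Blueprint that moves any actor overlapping its Capsule to the location and rotation of an Arrow component.
; The construction script places the Arrow from the TeleportLocation relative transform.
; On overlap, the actor's root component takes the Arrow's world location and rotation with a fixed enlarged scale.
; For player pawn 0, it also sets control rotation to the pawn's rotation, through LastHitBy rather than GetController.
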(event `self.Capsule.OnComponentBeginOverlap`
  (params (OverlappedComponent :type "PrimitiveComponent Object Reference") (OtherActor :type "Actor Object Reference") (OtherComp :type "PrimitiveComponent Object Reference") (OtherBodyIndex :type Integer) (bFromSweep :type Boolean) (SweepResult :type "HitResult Structure (by ref)"))
  (bind _returnvalue (`GameplayStatics.GetPlayerPawn` 0))
  (bind (_returnvalue_location _returnvalue_rotation) (`KismetMathLibrary.BreakTransform` (`SceneComponent.K2_GetComponentToWorld` (`self.Arrow`))))
  (`SceneComponent.K2_SetWorldTransform` (`Actor.RootComponent` OtherActor) (`KismetMathLibrary.MakeTransform` _returnvalue_location _returnvalue_rotation (1.5 1.5 1.5)) false false)
  (if (== OtherActor _returnvalue)
    (`Controller.SetControlRotation` (`Pawn.LastHitBy` (`GameplayStatics.GetPlayerPawn` 0)) (`self.K2_GetActorRotation` _returnvalue))))

(fn `UserConstructionScript`
  (`SceneComponent.K2_SetRelativeTransform` (`self.Arrow`) (`self.TeleportLocation`) false false))